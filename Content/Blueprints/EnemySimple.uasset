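; EnemySimple is an enemy Blueprint with a floating life bar, death effect and item drops.
; While its EnemyLife widget is active, Tick shows it and yaws and pitches it toward the player's follow camera.
; UpdateHUDLife feeds it the LifeStats ratio.
; GetKilled enables ragdoll physics and disables capsule collision, then timelines darken and dissolve the dynamic material, while DropItem spawns pickups with an outward impulse.
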(event `drop`
  (`self.DropItems`))

(event `self.ReceiveTick`
  (params (DeltaSeconds :type "Float (single-precision)"))
  (bind _widget (`self.Widget`))
  (bind _asenemy_life (cast `/Game/Blueprints/EnemyLife` (`WidgetComponent.GetUserWidgetObject` _widget)))
  (bind _ret (`/Game/Blueprints/EnemyLife.IsActive` _asenemy_life))
  (if _ret
    (`self.DisplayLife`)
    (`SceneComponent.SetHiddenInGame` _widget false false)
    (else
      (`SceneComponent.SetHiddenInGame` _widget true false))))

(event `self.ReceiveBeginPlay`
  (`self.UpdateHUDLife`))

(event `DisplayLife`
  (bind _widget (`self.Widget`))
  (bind _assurvival_wave_character (cast `SurvivalWaveCharacter` (`GameplayStatics.GetPlayerCharacter` 0)))
  (if (`KismetSystemLibrary.IsValid` _assurvival_wave_character)
    (bind (_returnvalue_roll _returnvalue_pitch _returnvalue_yaw) (`KismetMathLibrary.BreakRotator` (`KismetMathLibrary.FindLookAtRotation` (`SceneComponent.K2_GetComponentLocation` _widget) (`SceneComponent.K2_GetComponentLocation` (`SurvivalWaveCharacter.FollowCamera` _assurvival_wave_character)))))
    (`SceneComponent.K2_SetWorldRotation` _widget (`KismetMathLibrary.MakeRotator` 0.0 _returnvalue_pitch _returnvalue_yaw) false false)))

(event `self.UpdateHUDLife`
  (bind _lifestats (`self.LifeStats`))
  (bind _asenemy_life (cast `/Game/Blueprints/EnemyLife` (`WidgetComponent.GetUserWidgetObject` (`self.Widget`))))
  (bind _returnvalue (`LifeStat.GetLife` _lifestats))
  (bind _returnvalue_2 (`LifeStat.GetLifeMax` _lifestats))
  (`/Game/Blueprints/EnemyLife.UpdateLife` _asenemy_life (/ _returnvalue _returnvalue_2)))

(event `self.GetKilled`
  (`PrimitiveComponent.SetSimulatePhysics` (`self.Mesh`) true)
  (`PrimitiveComponent.SetCollisionEnabled` (`self.CapsuleComponent`) "NoCollision")
  (bind (_direction _driver) (`Timeline|FadeOut`)
    (:`Update`
      (`MaterialInstanceDynamic.SetVectorParameterValue` (`self.MatRef`) "BodyColor" (`KismetMathLibrary.LinearColorLerp` (`self.BodyColor`) (struct :`A` 1.0) _driver)))
    (:`Finished`
      (bind (_direction_2 _driver_2) (`Timeline|Dissolve`)
        (:`Update`
          (`MaterialInstanceDynamic.SetScalarParameterValue` (`self.MatRef`) "Dissolve" _driver_2))))))

(event `self.DropItem`
  (params (trans :type "Transform Structure") (drop :type "Item Structure"))
  (bind _returnvalue (`|SpawnActorFromClass` "/Game/Blueprints/ItemSpawn.ItemSpawn_C" trans "Undefined" "OverrideRootScale" null "/Game/Materials/TronAmmoL.TronAmmoL" null))
  (set `ItemPickup.ItemStat` drop _returnvalue)
  (`/Game/Blueprints/ItemSpawn.CheckItem` _returnvalue)
  (`PrimitiveComponent.AddImpulse` (`Pickup.PickupMesh` _returnvalue) (* (`KismetMathLibrary.Normal` (- (`self.K2_GetActorLocation` _returnvalue) (`self.K2_GetActorLocation`))) 200.0) "None" true))

(fn `UserConstructionScript`
  (bind _returnvalue (`PrimitiveComponent.CreateDynamicMaterialInstance` (`self.Mesh`) 0 "/Game/Materials/DissolveMannequin.DissolveMannequin"))
  (bind _output_get (set `self.MatRef` _returnvalue))
  (`MaterialInstanceDynamic.SetVectorParameterValue` _output_get "BodyColor" (`self.BodyColor`))
  (`MaterialInstanceDynamic.SetScalarParameterValue` _output_get "Dissolve" -0.2))
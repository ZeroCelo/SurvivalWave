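; One-shot button switch that, when a nearby player presses Interact, destroys a tagged actor and advances the shield talking actor's dialogue.
; The target is the first actor matching ActorTag, looked up on a short timer after BeginPlay.
; Box overlaps with SurvivalWaveCharacter gate the input and drive a timeline that slides and scales the prompt text.
; If a TalkingActorShieldBP exists, its text updates and the button's dynamic material switches on, locking the switch.
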(event `FindActor`
  (bind _outactors (`GameplayStatics.GetAllActorsWithTag` (`self.ActorTag`)))
  (if (> (`KismetArrayLibrary.Array_Length` _outactors) 0)
    (set `self.ActorRef` (`|GetArrayItem` _outactors))
    (`KismetSystemLibrary.PrintString` "Found Actor")))

(event `self.ReceiveBeginPlay`
  (`self.EnableInput` (`GameplayStatics.GetPlayerController` 0))
  (`self.AnimText` false)
  (`KismetSystemLibrary.K2_SetTimerDelegate` (delegate `FindActor`) 0.2))

(event `AnimText`
  (params (PlayForward :type Boolean))
  (bind _textrender (`self.TextRender`))
  (if PlayForward
    (bind (_direction _slidealpha) (`Timeline|TextSlide` :!label _label)
      (:`Update`
        (`SceneComponent.K2_SetRelativeLocation` _textrender (`KismetMathLibrary.VLerp` (`SceneComponent.RelativeLocation` (`self.TextStart`)) (`SceneComponent.RelativeLocation` (`self.TextEnd`)) _slidealpha) false false)
        (bind _returnvalue (+ 0.1 (* _slidealpha 0.9)))
        (`TextRenderComponent.SetXScale` _textrender _returnvalue)
        (`TextRenderComponent.SetYScale` _textrender _returnvalue)))
    (else
      (goto _label :!via `Reverse`))))

(event `self.Box.OnComponentBeginOverlap`
  (params (OverlappedComponent :type "PrimitiveComponent Object Reference") (OtherActor :type "Actor Object Reference") (OtherComp :type "PrimitiveComponent Object Reference") (OtherBodyIndex :type Integer) (bFromSweep :type Boolean) (SweepResult :type "HitResult Structure (by ref)"))
  (cast `SurvivalWaveCharacter` OtherActor)
  (`self.AnimText` true)
  (set `self.PlayerNear` true))

(event `self.Box.OnComponentEndOverlap`
  (params (OverlappedComponent :type "PrimitiveComponent Object Reference") (OtherActor :type "Actor Object Reference") (OtherComp :type "PrimitiveComponent Object Reference") (OtherBodyIndex :type Integer))
  (cast `SurvivalWaveCharacter` OtherActor)
  (`self.AnimText` false)
  (set `self.PlayerNear` false))

(event `InputAction|Interact` :consume false
  (params (Key :type "Key Structure"))
  (bind _actorref (`self.ActorRef`))
  (:`Pressed`
    (if (and (`self.PlayerNear`) (not (`self.SwitchOn`)))
      (`/Engine/EditorBlueprintResources/StandardMacros.IsValid` _actorref
        (:`Is Valid`
          (`self.K2_DestroyActor` _actorref)
          (bind _outactors (`GameplayStatics.GetAllActorsOfClass` "/Game/Blueprints/TalkingActorShieldBP.TalkingActorShieldBP_C"))
          (if (> (`KismetArrayLibrary.Array_Length` _outactors) 0)
            (bind _output (`|GetArrayItem` _outactors))
            (set `TalkingActor.CurrentTalkIndex` 2 _output)
            (`/Game/Blueprints/TalkingActorShieldBP.UpdateTextComponents` _output)
            (`/Game/Blueprints/TalkingActorShieldBP.ShowTextComponents` _output (`TalkingActor.bTextVisible` _output))
            (`MaterialInstanceDynamic.SetScalarParameterValue` (`self.ButtonMat`) "State" 1.0)
            (set `self.SwitchOn` true)))))))

(fn `UserConstructionScript`
  (bind _returnvalue (`PrimitiveComponent.CreateDynamicMaterialInstance` (`self.ButtonMesh`) 2 null))
  (set `self.ButtonMat` _returnvalue))
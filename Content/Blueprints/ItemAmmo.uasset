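; Pickup item Blueprint that sets its mesh's look for one of several life sizes or an ammo type.
; The construction script calls CheckItem, which switches on the ItemStat type to choose a Tron material and applies it to PickupMesh.
; CheckItem then toggles the mesh's physics and collision off and back on, leaving it simulating with query and physics collision.
; The file's event graph contains no overlap or collection logic.
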(event `self.ReceiveBeginPlay`)

(event `CheckItem`
  (bind _pickupmesh (`self.PickupMesh`))
  (switch `EItemType` (`.type` (break `Item` (`self.ItemStat`)))
    (:`IT_LifeS`
      (set `self.MaterialInstance` "/Game/Materials/TronLifeS.TronLifeS"))
    (:`IT_LifeM`
      (set `self.MaterialInstance` "/Game/Materials/TronLifeM.TronLifeM"))
    (:`IT_LifeL`
      (set `self.MaterialInstance` "/Game/Materials/TronLifeL.TronLifeL"))
    (:`IT_AmmoR`
      (set `self.MaterialInstance` "/Game/Materials/TronAmmo.TronAmmo")))
  (`PrimitiveComponent.SetMaterial` (`self.PickupMesh`) 0 (`self.MaterialInstance`))
  (`PrimitiveComponent.SetSimulatePhysics` _pickupmesh false)
  (`PrimitiveComponent.SetCollisionEnabled` _pickupmesh "NoCollision")
  (`PrimitiveComponent.SetCollisionEnabled` _pickupmesh "QueryAndPhysics")
  (`PrimitiveComponent.SetSimulatePhysics` _pickupmesh true))

(fn `UserConstructionScript`
  (`self.CheckItem`))
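; Key pickup actor that bobs and spins in the world; the file shows no collection logic.
; Two timelines restart themselves on finish, driving the pickup mesh's height around its starting Z and its yaw rotation.
; A SurvivalWaveCharacter entering the collision sphere raises the spin multiplier, and leaving resets it.
; The construction script creates a dynamic material on AnimMesh, using KeyValue as the hue of its glow color.
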(event `self.ReceiveBeginPlay`
  (bind (_returnvalue_x _returnvalue_y _returnvalue_z) (`KismetMathLibrary.BreakVector` (`SceneComponent.K2_GetComponentLocation` (`self.PickupMesh`))))
  (set `self.ZPos` _returnvalue_z)
  (`self.CallAnimation`)
  (`self.CallAnimation2`))

(event `CallAnimation`
  (bind _pickupmesh (`self.PickupMesh`))
  (bind (_returnvalue_x _returnvalue_y) (`KismetMathLibrary.BreakVector` (`SceneComponent.K2_GetComponentLocation` _pickupmesh)))
  (bind (_direction _translate) (`Timeline|Anim` :!via `PlayFromStart` :!label _label)
    (:`Update`
      (`SceneComponent.K2_SetWorldLocation` _pickupmesh (`KismetMathLibrary.MakeVector` _returnvalue_x _returnvalue_y (+ (`self.ZPos`) (* _translate 50.0))) false false))
    (:`Finished`
      (`self.CallAnimation`))))

(event `StopAnimation`
  (goto _label :!via `Stop`))

(event `CallAnimation2`
  (bind (_direction _rotate) (`Timeline|Anim2` :!via `PlayFromStart` :!label _label_2)
    (:`Update`
      (`SceneComponent.K2_SetWorldRotation` (`self.PickupMesh`) (`KismetMathLibrary.MakeRotator` 0.0 0.0 (* (* (`self.RotateSpeed`) _rotate) 360.0)) false false))
    (:`Finished`
      (`self.CallAnimation2`))))

(event `StopAnimation2`
  (goto _label_2 :!via `Stop`))

(event `self.CollisionSphere.OnComponentBeginOverlap`
  (params (OverlappedComponent :type "PrimitiveComponent Object Reference") (OtherActor :type "Actor Object Reference") (OtherComp :type "PrimitiveComponent Object Reference") (OtherBodyIndex :type Integer) (bFromSweep :type Boolean) (SweepResult :type "HitResult Structure (by ref)"))
  (cast `SurvivalWaveCharacter` OtherActor)
  (set `self.RotateSpeed` 4.0))

(event `self.CollisionSphere.OnComponentEndOverlap`
  (params (OverlappedComponent :type "PrimitiveComponent Object Reference") (OtherActor :type "Actor Object Reference") (OtherComp :type "PrimitiveComponent Object Reference") (OtherBodyIndex :type Integer))
  (cast `SurvivalWaveCharacter` OtherActor)
  (set `self.RotateSpeed` 1.0))

(fn `UserConstructionScript`
  (bind _returnvalue (`PrimitiveComponent.CreateDynamicMaterialInstance` (`self.AnimMesh`) 0 "/Game/Materials/KeyPickupMat.KeyPickupMat"))
  (bind _output_get (set `self.MatRef` _returnvalue))
  (`MaterialInstanceDynamic.SetVectorParameterValue` _output_get "GlowColor" (`KismetMathLibrary.HSVToRGB` (`self.KeyValue`) 1.0 1.0)))
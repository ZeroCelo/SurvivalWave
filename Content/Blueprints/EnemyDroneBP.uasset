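; Enemy drone Blueprint for the survival wave game that faces the player, shows a life-bar widget and drops pickups.
; Tick turns the sphere toward the player and, while the EnemyLife widget is active, aims it at the follow camera.
; A timeline lerps flight height, overlaps feed DetectDamage, and DropItem spawns an impulse-launched pickup.
; Death spawns an explosion and uses timelines on dynamic materials to fade the body dark, then burn it.
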(event `self.ReceiveBeginPlay`
  (`self.UpdateHUDLife`))

(event `self.ReceiveTick`
  (params (DeltaSeconds :type "Float (single-precision)"))
  (`self.DroneLook`)
  (`self.ShowLife`))

(event `DroneLook`
  (bind _assurvival_wave_character (cast `SurvivalWaveCharacter` (`GameplayStatics.GetPlayerCharacter` 0)))
  (if (`KismetSystemLibrary.IsValid` _assurvival_wave_character)
    (`SceneComponent.K2_SetRelativeRotation` (`self.Sphere`) (`KismetMathLibrary.ComposeRotators` (struct :`Yaw` 90.0) (`KismetMathLibrary.FindLookAtRotation` (`SceneComponent.K2_GetComponentLocation` (`self.CollisionSphere`)) (+ (`self.K2_GetActorLocation` _assurvival_wave_character) (0.0 0.0 30.0)))) false false)))

(event `self.UpdateFly`
  (params (pos :type "Float (single-precision)"))
  (bind _collisionsphere (`self.CollisionSphere`))
  (bind (_relativelocation_x _relativelocation_y _relativelocation_z) (`KismetMathLibrary.BreakVector` (`SceneComponent.RelativeLocation` _collisionsphere)))
  (bind (_direction _translate) (`Timeline|Flight` :!via `PlayFromStart`)
    (:`Update`
      (`SceneComponent.K2_SetRelativeLocation` _collisionsphere (`KismetMathLibrary.VLerp` (`KismetMathLibrary.MakeVector` 0.0 0.0 _relativelocation_z) (`KismetMathLibrary.MakeVector` 0.0 0.0 pos) _translate) false false))))

(event `DisplayLife`
  (bind _widget (`self.Widget`))
  (bind _assurvival_wave_character (cast `SurvivalWaveCharacter` (`GameplayStatics.GetPlayerCharacter` 0)))
  (if (`KismetSystemLibrary.IsValid` _assurvival_wave_character)
    (bind (_returnvalue_roll _returnvalue_pitch _returnvalue_yaw) (`KismetMathLibrary.BreakRotator` (`KismetMathLibrary.FindLookAtRotation` (`SceneComponent.K2_GetComponentLocation` _widget) (`SceneComponent.K2_GetComponentLocation` (`SurvivalWaveCharacter.FollowCamera` _assurvival_wave_character)))))
    (`SceneComponent.K2_SetRelativeRotation` _widget (`KismetMathLibrary.MakeRotator` 0.0 _returnvalue_pitch _returnvalue_yaw) false false)))

(event `ShowLife`
  (bind _widget (`self.Widget`))
  (bind _asenemy_life (cast `/Game/Blueprints/EnemyLife` (`WidgetComponent.GetUserWidgetObject` _widget)))
  (bind _ret (`/Game/Blueprints/EnemyLife.IsActive` _asenemy_life))
  (if _ret
    (`self.DisplayLife`)
    (`SceneComponent.SetHiddenInGame` _widget false false)
    (else
      (`SceneComponent.SetHiddenInGame` _widget true false))))

(event `self.UpdateHUDLife`
  (bind _lifestats (`self.LifeStats`))
  (bind _asenemy_life (cast `/Game/Blueprints/EnemyLife` (`WidgetComponent.GetUserWidgetObject` (`self.Widget`))))
  (bind _returnvalue (`LifeStat.GetLife` _lifestats))
  (bind _returnvalue_2 (`LifeStat.GetLifeMax` _lifestats))
  (`/Game/Blueprints/EnemyLife.UpdateLife` _asenemy_life (/ _returnvalue _returnvalue_2)))

(event `self.DropItem`
  (params (trans :type "Transform Structure") (drop :type "Item Structure"))
  (bind _returnvalue (`|SpawnActorFromClass` "/Game/Blueprints/ItemSpawn.ItemSpawn_C" trans "Undefined" "OverrideRootScale" null "/Game/Materials/TronAmmoL.TronAmmoL" null))
  (set `ItemPickup.ItemStat` drop _returnvalue)
  (`/Game/Blueprints/ItemSpawn.CheckItem` _returnvalue)
  (`PrimitiveComponent.AddImpulse` (`Pickup.PickupMesh` _returnvalue) (* (`KismetMathLibrary.Normal` (- (`self.K2_GetActorLocation` _returnvalue) (`self.K2_GetActorLocation`))) 100.0) "None" true))

(event `self.DeathBP`
  (`GameplayStatics.SpawnEmitterAtLocation` "/Game/ExampleContent/Blueprint_Communication/Effects/P_Explosion_Fireball.P_Explosion_Fireball" (`SceneComponent.K2_GetComponentLocation` (`self.CollisionSphere`))))

(event `self.GetKilled`
  (bind _dronemat (`self.DroneMat`))
  (bind _deathmat (`self.DeathMat`))
  (`PrimitiveComponent.SetCollisionEnabled` (`self.CollisionSphere`) "NoCollision")
  (bind (_direction _fade) (`Timeline|FadeOut`)
    (:`Update`
      (`MaterialInstanceDynamic.SetVectorParameterValue` _dronemat "BaseColor" (`KismetMathLibrary.LinearColorLerp` (`self.BodyColor`) (struct) _fade))
      (`MaterialInstanceDynamic.SetVectorParameterValue` _dronemat "GlowColor" (`KismetMathLibrary.LinearColorLerp` (`self.GlowColor`) (struct) _fade)))
    (:`Finished`
      (`PrimitiveComponent.SetMaterial` (`self.Sphere`) 0 (`self.DeathMat`))
      (bind (_direction_2 _glow _base) (`Timeline|Burn`)
        (:`Update`
          (`MaterialInstanceDynamic.SetVectorParameterValue` _deathmat "GlowColor" (`KismetMathLibrary.LinearColorLerp` (struct) (`self.DeathGlowColor`) _glow))
          (`MaterialInstanceDynamic.SetVectorParameterValue` _deathmat "BaseColor" (`KismetMathLibrary.LinearColorLerp` (`self.DeathBaseColor`) (struct :`R` 5.0 :`G` 2.083333 :`A` 1.0) _base)))))))

(event `self.CollisionSphere.OnComponentBeginOverlap`
  (params (OverlappedComponent :type "PrimitiveComponent Object Reference") (OtherActor :type "Actor Object Reference") (OtherComp :type "PrimitiveComponent Object Reference") (OtherBodyIndex :type Integer) (bFromSweep :type Boolean) (SweepResult :type "HitResult Structure (by ref)"))
  (`self.DetectDamage` OverlappedComponent OtherActor OtherComp OtherBodyIndex bFromSweep SweepResult))

(fn `UserConstructionScript`
  (bind _returnvalue (`PrimitiveComponent.CreateDynamicMaterialInstance` (`self.Sphere`) 0 "/Game/Materials/EnergyCore_Death.EnergyCore_Death"))
  (bind _output_get (set `self.DeathMat` _returnvalue))
  (bind _returnvalue_2 (`MaterialInstanceDynamic.K2_GetVectorParameterValue` _output_get "GlowColor"))
  (set `self.DeathGlowColor` _returnvalue_2)
  (bind _returnvalue_3 (`MaterialInstanceDynamic.K2_GetVectorParameterValue` _output_get "BaseColor"))
  (set `self.DeathBaseColor` _returnvalue_3)
  (bind _returnvalue_4 (`PrimitiveComponent.CreateDynamicMaterialInstance` (`self.Sphere`) 0 "/Game/Materials/DroneMat.DroneMat"))
  (bind _output_get_2 (set `self.DroneMat` _returnvalue_4))
  (`MaterialInstanceDynamic.SetVectorParameterValue` _output_get_2 "BaseColor" (`self.BodyColor`))
  (`MaterialInstanceDynamic.SetVectorParameterValue` _output_get_2 "GlowColor" (`self.GlowColor`)))
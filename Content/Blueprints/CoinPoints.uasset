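; A coin pickup that awards score points when the SurvivalWaveCharacter overlaps it, then destroys itself.
; On spawn it gets an impulse away from its owner and loops a timeline that spins the mesh.
; After a delay it turns off physics and homes toward the player pawn each tick at a set magnet speed.
; Overlap adds its points through SurvivalWaveGameMode.
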(event `ActivateMagnet`
  (set `self.PlayerMagnet` true)
  (`PrimitiveComponent.SetSimulatePhysics` (`self.Box`) false))

(event `self.ReceiveBeginPlay`
  (bind _returnvalue (`self.GetOwner`))
  (`|ExecutionSequence`
    (:`then_0`
      (if (`KismetSystemLibrary.IsValid` _returnvalue)
        (`PrimitiveComponent.AddImpulse` (`self.Box`) (* (`KismetMathLibrary.Normal` (- (`self.K2_GetActorLocation`) (`self.K2_GetActorLocation` _returnvalue))) 300.0) "None" true)))
    (:`then_1`
      (`KismetSystemLibrary.K2_SetTimerDelegate` (delegate `ActivateMagnet`) (`self.MagnetTime`))
      (`self.Animate`))))

(event `Animate`
  (bind (_direction _rotate) (`Timeline|Rotate` :!via `PlayFromStart`)
    (:`Update`
      (set `self.NewRotate` (`KismetMathLibrary.MakeRotator` 0.0 0.0 (* _rotate 360.0))))
    (:`Finished`
      (`self.Animate`))))

(event `self.ReceiveTick`
  (params (DeltaSeconds :type "Float (single-precision)"))
  (bind _returnvalue (`self.K2_GetActorLocation`))
  (bind _staticmesh (`self.StaticMesh`))
  (`SceneComponent.K2_SetWorldRotation` _staticmesh (`self.NewRotate`) false false)
  (`SceneComponent.SetWorldScale3D` _staticmesh (`KismetMathLibrary.MakeVector` 0.9 0.9 0.9))
  (if (`self.PlayerMagnet`)
    (`self.K2_SetActorLocation` (+ _returnvalue (* (`KismetMathLibrary.Normal` (- (`self.K2_GetActorLocation` (`GameplayStatics.GetPlayerPawn` 0)) _returnvalue)) (* (`self.MagnetImpulse`) DeltaSeconds))))))

(event `self.Box.OnComponentBeginOverlap`
  (params (OverlappedComponent :type "PrimitiveComponent Object Reference") (OtherActor :type "Actor Object Reference") (OtherComp :type "PrimitiveComponent Object Reference") (OtherBodyIndex :type Integer) (bFromSweep :type Boolean) (SweepResult :type "HitResult Structure (by ref)"))
  (cast `SurvivalWaveCharacter` OtherActor)
  (bind _assurvival_wave_game_mode (cast `SurvivalWaveGameMode` (`GameplayStatics.GetGameMode`)))
  (`SurvivalWaveGameMode.AddScore` _assurvival_wave_game_mode (`self.Points`))
  (`self.K2_DestroyActor`))

(fn `UserConstructionScript`)
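; Enemy dash drone pawn that drives the visuals and collision of a rolling, shielded sphere.
; A looping timer reads the AIDroneDashController state to set or blink the glow, overlapping pawns only during a dash.
; Tick rolls the mesh from planar velocity and toggles shield visibility, while timelines animate shield recharge and impact ripples through dynamic materials.
; Death disables collision, fades the colors to black, then swaps to a dissolve material.
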(event `BlinkChargeGlow`
  (bind _returnvalue (`self.GetController`))
  (`/Engine/EditorBlueprintResources/StandardMacros.DoOnce` false :!label _label
    (:`Completed`
      (bind (_direction _blink) (`Timeline|ChargeGlow` :!via `PlayFromStart`)
        (:`Update`
          (bind _asaidrone_dash_controller (cast `AIDroneDashController` _returnvalue))
          (if (`|EnumEquality` (`AIDroneDashController.DroneState` _asaidrone_dash_controller) "DS_Charge")
            (`MaterialInstanceDynamic.SetVectorParameterValue` (`self.DroneMatRef`) "GlowColor" (`KismetMathLibrary.LinearColorLerp` (`self.DroneGlowDash`) (struct) _blink))))
        (:`Finished`
          (bind _asaidrone_dash_controller_2 (cast `AIDroneDashController` _returnvalue))
          (`|ExecutionSequence`
            (:`then_0`
              (goto _label :!via `Reset`))
            (:`then_1`
              (if (`|EnumEquality` (`AIDroneDashController.DroneState` _asaidrone_dash_controller_2) "DS_Charge")
                (`self.BlinkChargeGlow`)))))))))

(event `UpdateColor`
  (bind _dronematref (`self.DroneMatRef`))
  (bind _collisionsphere (`self.CollisionSphere`))
  (bind _asaidrone_dash_controller (cast `AIDroneDashController` (`self.GetController`)))
  (switch `EDashState` (`AIDroneDashController.DroneState` _asaidrone_dash_controller)
    (:`DS_Moving`
      (`MaterialInstanceDynamic.SetVectorParameterValue` _dronematref "GlowColor" (`self.DroneGlowColor`))
      (`PrimitiveComponent.SetCollisionResponseToChannel` _collisionsphere "ECC_Pawn" "ECR_Ignore" :!label _label_2))
    (:`DS_Charge`
      (`self.BlinkChargeGlow`)
      (goto _label_2))
    (:`DS_Dash`
      (`MaterialInstanceDynamic.SetVectorParameterValue` _dronematref "GlowColor" (`self.DroneGlowDash`))
      (`PrimitiveComponent.SetCollisionResponseToChannel` _collisionsphere "ECC_Pawn" "ECR_Overlap"))
    (:`DS_Recharge`
      (`self.BlinkRecharge`)
      (goto _label_2))))

(event `self.ReceiveBeginPlay`
  (`MaterialInstanceDynamic.SetScalarParameterValue` (`self.ShieldMatRef`) "Recharge" 0.0)
  (`KismetSystemLibrary.K2_SetTimerDelegate` (delegate `UpdateColor`) 0.05 true))

(event `BlinkRecharge`
  (bind _returnvalue (`self.GetController`))
  (`/Engine/EditorBlueprintResources/StandardMacros.DoOnce` false :!label _label_3
    (:`Completed`
      (bind (_direction _blink) (`Timeline|RechargeGlow` :!via `PlayFromStart`)
        (:`Update`
          (bind _asaidrone_dash_controller (cast `AIDroneDashController` _returnvalue))
          (if (`|EnumEquality` (`AIDroneDashController.DroneState` _asaidrone_dash_controller) "DS_Recharge")
            (`MaterialInstanceDynamic.SetVectorParameterValue` (`self.DroneMatRef`) "GlowColor" (`KismetMathLibrary.LinearColorLerp` (`self.DroneGlowRecharge`) (struct) _blink))))
        (:`Finished`
          (bind _asaidrone_dash_controller_2 (cast `AIDroneDashController` _returnvalue))
          (`|ExecutionSequence`
            (:`then_0`
              (goto _label_3 :!via `Reset`))
            (:`then_1`
              (if (`|EnumEquality` (`AIDroneDashController.DroneState` _asaidrone_dash_controller_2) "DS_Recharge")
                (`self.BlinkRecharge`)))))))))

(event `self.ReceiveTick`
  (params (DeltaSeconds :type "Float (single-precision)"))
  (`self.UpdateMoveAnim`)
  (`self.UpdateShieldCull`))

(event `UpdateDamageCollision`)

(event `UpdateMoveAnim`
  (bind (_returnvalue_x _returnvalue_y) (`KismetMathLibrary.BreakVector` (`self.GetVelocity`)))
  (bind _rotationamount (`self.RotationAmount`))
  (bind _returnvalue (`KismetMathLibrary.MakeVector` _returnvalue_x _returnvalue_y))
  (bind _returnvalue_2 (`KismetMathLibrary.VSize` _returnvalue))
  (if (> _returnvalue_2 0.0)
    (set `self.RotationAmount` (+ (`self.RotationAmount`) (* (/ _returnvalue_2 (* (`KismetMathLibrary.GetPI`) (/ (`SphereComponent.SphereRadius` (`self.CollisionSphere`)) 135.0))) (`GameplayStatics.GetWorldDeltaSeconds`))))
    (`SceneComponent.K2_SetWorldRotation` (`self.DroneSphere`) (`KismetMathLibrary.RotatorFromAxisAndAngle` (`KismetMathLibrary.GetRightVector` (`KismetMathLibrary.MakeRotFromX` (`KismetMathLibrary.Normal` _returnvalue))) (`self.RotationAmount`)) false false)
    (if (> _rotationamount 360.0)
      (set `self.RotationAmount` (- _rotationamount 360.0)))))

(event `self.GetHit`
  (params (HitResult :type "HitResult Structure"))
  (bind (_bblockinghit _binitialoverlap _time _distance _location _impactpoint) (`GameplayStatics.BreakHitResult` HitResult))
  (if _bblockinghit
    (set `self.HitDir` (- _impactpoint (`self.K2_GetActorLocation`)))
    (`self.ShieldHitAnim`)))

(event `UpdateShieldCull`
  (bind _returnvalue (`LifeStat.IsShieldActive` (`self.LifeStats`)))
  (if _returnvalue
    (bind _returnvalue_2 (`LifeStat.IsShieldRecharging` (`self.LifeStats`)))
    (if (or _returnvalue_2 (`self.ShieldDmg`) (`self.ShieldCharging`))
      (`SceneComponent.SetHiddenInGame` (`self.ShieldSphere`) false false)
      (`self.ShieldRechargeAnim`)
      (else
        (`SceneComponent.SetHiddenInGame` (`self.ShieldSphere`) true false)
        (`self.ShieldRechargeAnim`)))
    (else
      (`SceneComponent.SetHiddenInGame` (`self.ShieldSphere`) true false))))

(event `self.CollisionSphere.OnComponentEndOverlap`
  (params (OverlappedComponent :type "PrimitiveComponent Object Reference") (OtherActor :type "Actor Object Reference") (OtherComp :type "PrimitiveComponent Object Reference") (OtherBodyIndex :type Integer))
  (bind _asprojectile (cast `Projectile` OtherActor))
  (bind _returnvalue (`LifeStat.IsShieldActive` (`self.LifeStats`)))
  (if _returnvalue
    (set `self.HitDir` (- (`self.K2_GetActorLocation` _asprojectile) (`self.K2_GetActorLocation`)))
    (`self.ShieldHitAnim`)))

(event `ShieldRechargeAnim`
  (set `self.ShieldCharging` true)
  (bind _returnvalue (`LifeStat.IsShieldRecharging` (`self.LifeStats`)))
  (if _returnvalue
    (bind (_direction _charge) (`Timeline|ShieldRecharge` :!label _label_4)
      (:`Update`
        (`MaterialInstanceDynamic.SetScalarParameterValue` (`self.ShieldMatRef`) "Recharge" _charge))
      (:`Finished`
        (set `self.ShieldCharging` false)))
    (else
      (goto _label_4 :!via `Reverse`))))

(event `ShieldHitAnim`
  (bind _shieldmatref (`self.ShieldMatRef`))
  (set `self.ShieldDmg` true)
  (bind (_direction _radius) (`Timeline|ShieldHit` :!via `PlayFromStart`)
    (:`Update`
      (`MaterialInstanceDynamic.SetScalarParameterValue` _shieldmatref "HitRadius" (* _radius 75.0))
      (`MaterialInstanceDynamic.SetVectorParameterValue` _shieldmatref "HitPos" (`KismetMathLibrary.Conv_VectorToLinearColor` (+ (`self.K2_GetActorLocation`) (`self.HitDir`)))))
    (:`Finished`
      (`MaterialInstanceDynamic.SetScalarParameterValue` _shieldmatref "HitRadius" 0.0)
      (set `self.ShieldDmg` false))))

(event `self.GetKilled`
  (bind _dronematref (`self.DroneMatRef`))
  (bind _dronematref_2 (`self.DroneMatRef`))
  (`PrimitiveComponent.SetCollisionEnabled` (`self.CollisionSphere`) "NoCollision")
  (bind _returnvalue (`MaterialInstanceDynamic.K2_GetVectorParameterValue` _dronematref "BaseColor"))
  (set `self.DroneBaseColor` _returnvalue)
  (bind _returnvalue_2 (`MaterialInstanceDynamic.K2_GetVectorParameterValue` _dronematref "GlowColor"))
  (set `self.DroneGlowColor` _returnvalue_2)
  (bind (_direction _fade) (`Timeline|FadeOut` :!via `PlayFromStart`)
    (:`Update`
      (`MaterialInstanceDynamic.SetVectorParameterValue` _dronematref_2 "BaseColor" (`KismetMathLibrary.LinearColorLerp` (`self.DroneBaseColor`) (struct) _fade))
      (`MaterialInstanceDynamic.SetVectorParameterValue` _dronematref_2 "GlowColor" (`KismetMathLibrary.LinearColorLerp` (`self.DroneGlowColor`) (struct) _fade)))
    (:`Finished`
      (`PrimitiveComponent.SetMaterial` (`self.DroneSphere`) 0 (`self.DeathMatRef`))
      (bind (_direction_2 _dissolveamount) (`Timeline|Dissolve` :!via `PlayFromStart`)
        (:`Update`
          (`MaterialInstanceDynamic.SetScalarParameterValue` (`self.DeathMatRef`) "Dissolve" _dissolveamount))))))

(event `self.CollisionSphere.OnComponentBeginOverlap`
  (params (OverlappedComponent :type "PrimitiveComponent Object Reference") (OtherActor :type "Actor Object Reference") (OtherComp :type "PrimitiveComponent Object Reference") (OtherBodyIndex :type Integer) (bFromSweep :type Boolean) (SweepResult :type "HitResult Structure (by ref)"))
  (cast `EnemyDrone` OtherActor
    (:`CastFailed`
      (cast `EnemyCharacter` OtherActor
        (:`CastFailed`
          (bind _assurvival_char_bp (cast `/Game/Blueprints/SurvivalChar_BP` OtherActor)
            (:`then`
              (bind _returnvalue (+ (`self.K2_GetActorLocation` _assurvival_char_bp) (0.0 0.0 50.0)))
              (`/Game/Blueprints/SurvivalChar_BP.ShieldHitAnim` _assurvival_char_bp (+ _returnvalue (* (`KismetMathLibrary.Normal` (- (`self.K2_GetActorLocation`) _returnvalue)) (`CapsuleComponent.CapsuleRadius` (`Character.CapsuleComponent` _assurvival_char_bp))))))
            (:`CastFailed`
              (`self.DetectDamage` OverlappedComponent OtherActor OtherComp OtherBodyIndex bFromSweep SweepResult))))))))

(fn `UserConstructionScript`
  (bind _dronesphere (`self.DroneSphere`))
  (bind _sphereradius (`SphereComponent.SphereRadius` (`self.CollisionSphere`)))
  (bind _returnvalue (/ _sphereradius 50.0))
  (bind _returnvalue_2 (+ _returnvalue 0.05))
  (`CapsuleComponent.SetCapsuleRadius` (`self.CapsuleComponent`) _sphereradius true)
  (`SceneComponent.SetRelativeScale3D` (`self.DroneSphere`) (`KismetMathLibrary.MakeVector` _returnvalue _returnvalue _returnvalue))
  (`SceneComponent.SetRelativeScale3D` (`self.ShieldSphere`) (`KismetMathLibrary.MakeVector` _returnvalue_2 _returnvalue_2 _returnvalue_2))
  (bind _returnvalue_3 (`PrimitiveComponent.CreateDynamicMaterialInstance` (`self.ShieldSphere`) 0 null))
  (bind _output_get (set `self.ShieldMatRef` _returnvalue_3))
  (`MaterialInstanceDynamic.SetVectorParameterValue` _output_get "BaseColor" (`self.ShieldColor`))
  (bind _returnvalue_4 (`PrimitiveComponent.CreateDynamicMaterialInstance` _dronesphere 0 "/Game/Materials/DissolveMat_Inst.DissolveMat_Inst"))
  (set `self.DeathMatRef` _returnvalue_4)
  (bind _returnvalue_5 (`PrimitiveComponent.CreateDynamicMaterialInstance` _dronesphere 0 "/Game/Materials/DroneMat4.DroneMat4"))
  (bind _output_get_2 (set `self.DroneMatRef` _returnvalue_5))
  (bind _returnvalue_6 (`MaterialInstanceDynamic.K2_GetVectorParameterValue` _output_get_2 "GlowColor"))
  (set `self.DroneGlowColor` _returnvalue_6))
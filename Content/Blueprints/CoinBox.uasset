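; CoinBox is a loot box actor that bursts into coin pickups when a SurvivalWaveCharacter overlaps its box component.
; A one-time drop spawns CoinCount CoinPoints actors at random points above the box and pushes them away with velocity-change impulses.
; The Opening timeline pitches LootBoxArrow and repeatedly multiplies actor scale by its Disappear track, then destroys the box when finished.
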(event `OpenBox`
  (`self.DropCoins`)
  (bind (_direction _rotate _disappear) (`Timeline|Opening`)
    (:`Update`
      (`SceneComponent.K2_SetRelativeRotation` (`self.LootBoxArrow`) (`KismetMathLibrary.MakeRotator` 0.0 (* _rotate 100.0) 90.0) false false)
      (`self.SetActorScale3D` (* (`self.GetActorScale3D`) _disappear)))
    (:`Finished`
      (`self.KillBox`))))

(event `KillBox`
  (`self.K2_DestroyActor`))

(event `self.Box.OnComponentBeginOverlap`
  (params (OverlappedComponent :type "PrimitiveComponent Object Reference") (OtherActor :type "Actor Object Reference") (OtherComp :type "PrimitiveComponent Object Reference") (OtherBodyIndex :type Integer) (bFromSweep :type Boolean) (SweepResult :type "HitResult Structure (by ref)"))
  (if (`KismetSystemLibrary.IsValid` OtherActor)
    (cast `SurvivalWaveCharacter` OtherActor)
    (`self.OpenBox`)))

(event `DropCoins`
  (`/Engine/EditorBlueprintResources/StandardMacros.DoOnce` false
    (:`Completed`
      (for _ (range (`self.CoinCount`))
        (bind _returnvalue (`|SpawnActorFromClass` "/Game/Blueprints/CoinPoints.CoinPoints_C" (`KismetMathLibrary.Conv_VectorToTransform` (`KismetMathLibrary.RandomPointInBoundingBox` (+ (`SceneComponent.K2_GetComponentLocation` (`self.RootBox`)) (0.0 0.0 60.0)) (`KismetMathLibrary.MakeVector` 10.0 10.0 50.0))) "Undefined" "OverrideRootScale" self))
        (bind _box (`/Game/Blueprints/CoinPoints.Box` _returnvalue))
        (`PrimitiveComponent.AddImpulse` _box (* (`KismetMathLibrary.Normal` (- (`SceneComponent.K2_GetComponentLocation` _box) (`self.K2_GetActorLocation`))) 200.0) "None" true)))))

(fn `UserConstructionScript`)
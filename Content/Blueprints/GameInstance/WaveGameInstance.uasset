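; Game instance that manages menu display: pause, options and advanced graphics widgets, plus loading the main menu level.
; Each widget is created on first use and cached, and showing or hiding the pause menu also switches cursor visibility and input mode.
; Leaving visual settings branches on InGame, either showing the paused-game options menu or telling MainMenuMode to hide graphics.
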(event `HideVisual`
  ;[1 1 1] Hides Visual Settings and Display Correct Menu
  (if (`self.InGame`)
    (`self.ShowOptionsMenu`)
    (else
      (bind _asmain_menu_mode (cast `/Game/Blueprints/MainMenu/MainMenuMode` (`GameplayStatics.GetGameMode`)))
      (`/Game/Blueprints/MainMenu/MainMenuMode.HideGraphics` _asmain_menu_mode))))

(event `ShowVisualMenu`
  ;[1 1 1] Show Advanced Graphics Settings
  (`/Engine/EditorBlueprintResources/StandardMacros.IsValid` (`self.MenuGraphics`)
    (:`Is Valid`
      _)
    (:`Is Not Valid`
      (bind _returnvalue (`|CreateWidget` "/Game/Blueprints/GameInstance/GraphicsMenu.GraphicsMenu_C"))
      (set `self.MenuGraphics` _returnvalue)))
  (`UserWidget.AddToViewport` (`self.MenuGraphics`) 0))

(event `LaunchMainMenu`
  ;[1 1 1] Load main menu
  (`GameplayStatics.OpenLevel` "MainMenuPersist"))

(event `ShowPauseMenu`
  (bind _returnvalue (`GameplayStatics.GetPlayerController` 0))
  ;[1 1 1] Display Pause Menu In gameplay
  (if (not (`KismetSystemLibrary.IsValid` (`self.MenuPause`)))
    (bind _returnvalue_2 (`|CreateWidget` "/Game/Blueprints/GameInstance/PauseMenu.PauseMenu_C" (`GameplayStatics.GetPlayerController` 0)))
    (set `self.MenuPause` _returnvalue_2))
  (`UserWidget.AddToViewport` (`self.MenuPause`) 0)
  (set `PlayerController.bShowMouseCursor` true _returnvalue)
  (`WidgetBlueprintLibrary.SetInputMode_GameAndUIEx` _returnvalue))

(event `ShowOptionsMenu`
  ;[1 1 1] Show Options Menu in Paused Game
  (if (not (`KismetSystemLibrary.IsValid` (`self.MenuOptions`)))
    (bind _returnvalue (`|CreateWidget` "/Game/Blueprints/GameInstance/PauseOptionsMenu.PauseOptionsMenu_C"))
    (set `self.MenuOptions` _returnvalue))
  (`UserWidget.AddToViewport` (`self.MenuOptions`) 0))

(event `HidePauseMenu`
  (bind _returnvalue (`GameplayStatics.GetPlayerController` 0))
  (bind _menuoptions (`self.MenuOptions`))
  ;[1 1 1] Hide Pause Menu
  (if (not (`KismetSystemLibrary.IsValid` (`self.MenuPause`)))
    (bind _returnvalue_2 (`|CreateWidget` "/Game/Blueprints/GameInstance/PauseMenu.PauseMenu_C" (`GameplayStatics.GetPlayerController` 0)))
    (set `self.MenuPause` _returnvalue_2))
  (`Widget.RemoveFromParent` (`self.MenuPause`))
  (set `PlayerController.bShowMouseCursor` false _returnvalue)
  (`WidgetBlueprintLibrary.SetInputMode_GameOnly` _returnvalue)
  (`/Engine/EditorBlueprintResources/StandardMacros.IsValid` _menuoptions
    (:`Is Valid`
      (`Widget.RemoveFromParent` _menuoptions))))
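; Boss enemy for the survival wave game, with a floating life-bar widget, overlap-based damage detection and a death effect.
; Each tick the widget turns to face the player's follow camera, and UpdateHUDLife feeds it the life ratio from LifeStats.
; Capsule overlaps are forwarded to DetectDamage.
; GetKilled disables capsule collision, then chains timelines on a construction-time dynamic material, fading BossColor to black before dissolving the mesh.
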(event `self.ReceiveTick`
  (params (DeltaSeconds :type "Float (single-precision)"))
  (`self.DisplayLife`))

(event `self.GetKilled`
  (`PrimitiveComponent.SetCollisionEnabled` (`self.CapsuleComponent`) "NoCollision")
  (bind (_direction _driver) (`Timeline|Fade`)
    (:`Update`
      (`MaterialInstanceDynamic.SetVectorParameterValue` (`self.MatRef`) "BodyColor" (`KismetMathLibrary.LinearColorLerp` (`self.BossColor`) (struct :`A` 1.0) _driver)))
    (:`Finished`
      (bind (_direction_2 _driver_2) (`Timeline|Dissolve`)
        (:`Update`
          (`MaterialInstanceDynamic.SetScalarParameterValue` (`self.MatRef`) "Dissolve" _driver_2))))))

(event `DisplayLife`
  (bind _widget (`self.Widget`))
  (bind _assurvival_wave_character (cast `SurvivalWaveCharacter` (`GameplayStatics.GetPlayerCharacter` 0)))
  (if (`KismetSystemLibrary.IsValid` _assurvival_wave_character)
    (bind (_returnvalue_roll _returnvalue_pitch _returnvalue_yaw) (`KismetMathLibrary.BreakRotator` (`KismetMathLibrary.FindLookAtRotation` (`SceneComponent.K2_GetComponentLocation` _widget) (`SceneComponent.K2_GetComponentLocation` (`SurvivalWaveCharacter.FollowCamera` _assurvival_wave_character)))))
    (`SceneComponent.K2_SetWorldRotation` _widget (`KismetMathLibrary.MakeRotator` 0.0 _returnvalue_pitch _returnvalue_yaw) false false)))

(event `self.UpdateHUDLife`
  (bind _lifestats (`self.LifeStats`))
  (bind _asenemy_life (cast `/Game/Blueprints/EnemyLife` (`WidgetComponent.GetUserWidgetObject` (`self.Widget`))))
  (bind _returnvalue (`LifeStat.GetLife` _lifestats))
  (bind _returnvalue_2 (`LifeStat.GetLifeMax` _lifestats))
  (`/Game/Blueprints/EnemyLife.UpdateLife` _asenemy_life (/ _returnvalue _returnvalue_2)))

(event `self.CapsuleComponent.OnComponentBeginOverlap`
  (params (OverlappedComponent :type "PrimitiveComponent Object Reference") (OtherActor :type "Actor Object Reference") (OtherComp :type "PrimitiveComponent Object Reference") (OtherBodyIndex :type Integer) (bFromSweep :type Boolean) (SweepResult :type "HitResult Structure (by ref)"))
  (`self.DetectDamage` OverlappedComponent OtherActor OtherComp OtherBodyIndex bFromSweep SweepResult))

(fn `UserConstructionScript`
  (bind _matref (`self.MatRef`))
  (bind _returnvalue (`PrimitiveComponent.CreateDynamicMaterialInstance` (`self.Mesh`) 0 "/Game/Materials/DissolveMannequin.DissolveMannequin"))
  (set `self.MatRef` _returnvalue)
  (`MaterialInstanceDynamic.SetVectorParameterValue` _matref "BodyColor" (`self.BossColor`))
  (`MaterialInstanceDynamic.SetScalarParameterValue` _matref "Dissolve" -0.2))
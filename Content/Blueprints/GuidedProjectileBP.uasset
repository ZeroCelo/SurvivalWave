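; Guided projectile that visually travels out from its owner, then homes in on the player character.
; On BeginPlay, if it has a valid owner, the Moving timeline lerps FXPoint from the owner's current location to that component's initial world position.
; When the timeline finishes, ProjectileMove switches to homing, targeting the capsule of player 0's character.
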(event `self.ReceiveBeginPlay`
  (set `self.FXStart` (`SceneComponent.K2_GetComponentLocation` (`self.FXPoint`)))
  (if (`KismetSystemLibrary.IsValid` (`self.GetOwner`))
    (`self.ShowProjectile`)))

(event `ShowProjectile`
  (bind _returnvalue (`GameplayStatics.GetPlayerCharacter` 0))
  (bind _projectilemove (`self.ProjectileMove`))
  (bind (_direction _translate) (`Timeline|Moving`)
    (:`Update`
      (`SceneComponent.K2_SetWorldLocation` (`self.FXPoint`) (`KismetMathLibrary.VLerp` (`self.K2_GetActorLocation` (`self.GetOwner`)) (`self.FXStart`) _translate) false false))
    (:`Finished`
      (if (`KismetSystemLibrary.IsValid` _returnvalue)
        (set `ProjectileMovementComponent.HomingTargetComponent` (`Character.CapsuleComponent` _returnvalue) _projectilemove)
        (set `ProjectileMovementComponent.bIsHomingProjectile` true _projectilemove)))))

(fn `UserConstructionScript`)
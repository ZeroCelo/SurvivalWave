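; Sliding double door for the survival wave game that opens for nearby characters and can lock behind them.
; A Box trigger counts overlapping SurvivalWaveCharacters, driving the Opening timeline to slide the panels and spin the lock, reversing it when none remain.
; When the last one exits on the door's forward-facing side, a direction-vector check clears Active, blocking reopening.
; The lock's material reflects open, ready or locked state.
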(event `OpenDoor`
  (if (and (`self.DoorClosed`) (`self.Active`))
    (`PrimitiveComponent.SetMaterial` (`self.Lock`) 0 "/Game/DemoRoom/Materials/M_UE4_Logo_Doors.M_UE4_Logo_Doors")
    (bind (_direction _move _rotate) (`Timeline|Opening` :!label _label)
      (:`Update`
        (`|ExecutionSequence`
          (:`then_0`
            (bind _returnvalue (* _move 220.0))
            (`SceneComponent.K2_SetRelativeLocation` (`self.LeftDoor`) (`KismetMathLibrary.MakeVector` 0.0 _returnvalue) false false)
            (`SceneComponent.K2_SetRelativeLocation` (`self.RightDoor`) (`KismetMathLibrary.MakeVector` 0.0 (* _returnvalue -1.0)) false false))
          (:`then_1`
            (`SceneComponent.K2_SetRelativeRotation` (`self.Lock`) (`KismetMathLibrary.MakeRotator` (* _rotate 90.0)) false false))))
      (:`Finished`
        (if (`|EnumEquality` _direction "Backward")
          (`self.CheckActive`))))))

(event `CloseDoor`
  (goto _label :!via `Reverse`))

(event `self.ReceiveBeginPlay`)

(event `CheckActive`
  (bind _lock (`self.Lock`))
  (if (`self.Active`)
    (`PrimitiveComponent.SetMaterial` _lock 0 "/Game/DemoRoom/Materials/M_UE4_Logo_Door.M_UE4_Logo_Door")
    (else
      (`PrimitiveComponent.SetMaterial` _lock 0 "/Game/DemoRoom/Materials/M_UE4_Logo_Door_Lock.M_UE4_Logo_Door_Lock"))))

(event `self.Box.OnComponentBeginOverlap`
  (params (OverlappedComponent :type "PrimitiveComponent Object Reference") (OtherActor :type "Actor Object Reference") (OtherComp :type "PrimitiveComponent Object Reference") (OtherBodyIndex :type Integer) (bFromSweep :type Boolean) (SweepResult :type "HitResult Structure (by ref)"))
  (bind _assurvival_wave_character (cast `SurvivalWaveCharacter` OtherActor))
  (set `self.PlayerNear` (+ (`self.PlayerNear`) 1))
  (`self.CheckPlayer` _assurvival_wave_character))

(event `self.Box.OnComponentEndOverlap`
  (params (OverlappedComponent :type "PrimitiveComponent Object Reference") (OtherActor :type "Actor Object Reference") (OtherComp :type "PrimitiveComponent Object Reference") (OtherBodyIndex :type Integer))
  (bind _assurvival_wave_character (cast `SurvivalWaveCharacter` OtherActor))
  (set `self.PlayerNear` (- (`self.PlayerNear`) 1))
  (`self.CheckPlayer` _assurvival_wave_character))

(event `CheckPlayer`
  (params (Player :type "SurvivalWaveCharacter Object Reference"))
  (if (<= (`self.PlayerNear`) 0)
    (`|ExecutionSequence`
      (:`then_1`
        (`self.CloseDoor`)
        (if (`KismetSystemLibrary.IsValid` Player)
          (if (> (`KismetMathLibrary.VSize` (- (`self.GetActorForwardVector`) (`KismetMathLibrary.Normal` (- (`self.K2_GetActorLocation`) (`self.K2_GetActorLocation` Player))))) 1.45)
            (set `self.Active` false)
            (`self.CheckActive`)))))
    (else
      (`self.OpenDoor`))))

(fn `UserConstructionScript`
  (`self.CheckActive`))
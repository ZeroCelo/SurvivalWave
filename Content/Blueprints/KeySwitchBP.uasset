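; Key switch actor whose mesh color identifies its key value, with a flag that follows the game's color-blind setting.
; The construction script gives the switch mesh a dynamic material and sets its base color from KeyValue as a fully saturated hue.
; At runtime, a one-second looping timer copies the ColorBlind setting from WaveGameInstance into DisplayKey, so changes are picked up without using Tick.
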(event `SetupColorBlind`
  (bind _aswave_game_instance (cast `/Game/Blueprints/GameInstance/WaveGameInstance` (`GameplayStatics.GetGameInstance`)))
  (set `self.bDisplayKey` (`/Game/Blueprints/GameInstance/WaveGameInstance.ColorBlind` _aswave_game_instance)))

(event `self.ReceiveBeginPlay`
  (`KismetSystemLibrary.K2_SetTimerDelegate` (delegate `SetupColorBlind`) 1.0 true))

(fn `UserConstructionScript`
  (bind _returnvalue (`PrimitiveComponent.CreateDynamicMaterialInstance` (`self.SwitchMesh`) 0 "/Game/Materials/KeySwitchMat_Inst.KeySwitchMat_Inst"))
  (bind _output_get (set `self.MatRef` _returnvalue))
  (`MaterialInstanceDynamic.SetVectorParameterValue` _output_get "BaseColor" (`KismetMathLibrary.HSVToRGB` (`self.KeyValue`) 1.0 1.0)))
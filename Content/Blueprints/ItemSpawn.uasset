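; ItemSpawn is a pickup item actor for health, ammo and gun types, configured by ItemStat.Type.
; Its construction script fills per-type material, mesh, size and limit maps, then runs CheckItem.
; CheckItem applies mesh, scale and material with fallbacks for unmapped types, such as a cube mesh, resets collision and physics simulation, and calls CheckLimit.
; BeginPlay calls CheckLimit again; its body is not defined in these graphs.
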(event `self.CheckItem`
  (`self.CheckItemMesh`)
  (`self.CheckItemSize`)
  (`self.CheckItemMaterial`)
  (`self.CheckCollision`)
  (`self.CheckLimit`))

(event `self.ReceiveBeginPlay`
  (`self.CheckLimit`))

(event `CheckItemMaterial`
  (bind _pickupmesh (`self.PickupMesh`))
  (bind _type (break `Item` (`self.ItemStat`)))
  (bind _returnvalue (`self.ItemMapContainsMaterial` _type))
  (if _returnvalue
    (bind _returnvalue_2 (`self.ItemMapGetMaterial` _type))
    (set `self.MaterialInstance` _returnvalue_2)
    (`PrimitiveComponent.SetMaterial` (`self.PickupMesh`) 0 (`self.MaterialInstance`))
    (else
      (for (_ _array_index) (`MeshComponent.GetMaterials` _pickupmesh)
        (`PrimitiveComponent.SetMaterial` _pickupmesh _array_index null)))))

(event `CheckCollision`
  (bind _pickupmesh (`self.PickupMesh`))
  (`PrimitiveComponent.SetSimulatePhysics` _pickupmesh false)
  (`PrimitiveComponent.SetCollisionEnabled` _pickupmesh "NoCollision")
  (`PrimitiveComponent.SetCollisionEnabled` _pickupmesh "QueryAndPhysics")
  (`PrimitiveComponent.SetSimulatePhysics` _pickupmesh true))

(event `CheckItemMesh`
  (bind _pickupmesh (`self.PickupMesh`))
  (bind _type (break `Item` (`self.ItemStat`)))
  (bind _returnvalue (`self.ItemMapContainsMesh` _type))
  (if _returnvalue
    (bind _returnvalue_2 (`self.ItemMapGetMesh` _type))
    (`StaticMeshComponent.SetStaticMesh` _pickupmesh _returnvalue_2)
    (else
      (`StaticMeshComponent.SetStaticMesh` _pickupmesh "/Game/StarterContent/Shapes/Shape_Cube.Shape_Cube"))))

(event `CheckItemSize`
  (bind _pickupmesh (`self.PickupMesh`))
  (bind _type (break `Item` (`self.ItemStat`)))
  (bind _returnvalue (`self.ItemMapContainsSize` _type))
  (if _returnvalue
    (bind _returnvalue_2 (`self.ItemMapGetSize` _type))
    (`SceneComponent.SetRelativeScale3D` _pickupmesh _returnvalue_2)
    (else
      (`SceneComponent.SetRelativeScale3D` _pickupmesh (1.0 1.0 1.0)))))

(event `SetupMapAll`
  (`self.SetupMapMaterial`)
  (`self.SetupMapMesh`)
  (`self.SetupMapSize`)
  (`self.SetupMapLimit`))

(event `SetupMapMaterial`
  (`|ExecutionSequence`
    (:`then_0`
      (`self.ItemMapAddMaterial` "IT_LifeS" "/Game/Materials/TronLifeS.TronLifeS"))
    (:`then_1`
      (`self.ItemMapAddMaterial` "IT_LifeM" "/Game/Materials/TronLifeM.TronLifeM"))
    (:`then_2`
      (`self.ItemMapAddMaterial` "IT_LifeL" "/Game/Materials/TronLifeL.TronLifeL"))
    (:`then_3`
      (`self.ItemMapAddMaterial` "IT_AmmoR" "/Game/Materials/TronAmmo.TronAmmo"))
    (:`then_4`
      (`self.ItemMapAddMaterial` "IT_AmmoL" "/Game/Materials/TronAmmoL.TronAmmoL"))))

(event `SetupMapMesh`
  (`|ExecutionSequence`
    (:`then_0`
      (`self.ItemMapAddMesh` "IT_GunR" "/Game/Weapons/RifleStatic.RifleStatic"))
    (:`then_1`
      (`self.ItemMapAddMesh` "IT_GunL" "/Game/Weapons/LauncherStatic.LauncherStatic"))))

(event `SetupMapSize`
  (bind _returnvalue (`KismetMathLibrary.MakeVector` 0.5 0.5 0.5))
  (`|ExecutionSequence`
    (:`then_0`
      (`self.ItemMapAddSize` "IT_LifeS" _returnvalue))
    (:`then_1`
      (`self.ItemMapAddSize` "IT_LifeM" _returnvalue))
    (:`then_2`
      (`self.ItemMapAddSize` "IT_LifeL" _returnvalue))
    (:`then_3`
      (`self.ItemMapAddSize` "IT_AmmoR" _returnvalue))
    (:`then_4`
      (`self.ItemMapAddSize` "IT_AmmoL" _returnvalue))))

(event `SetupMapLimit`
  (`|ExecutionSequence`
    (:`then_0`
      (`self.ItemMapAddLimit` "IT_LifeS" 1))
    (:`then_1`
      (`self.ItemMapAddLimit` "IT_LifeM" 1))
    (:`then_2`
      (`self.ItemMapAddLimit` "IT_LifeL" 1))
    (:`then_3`
      (`self.ItemMapAddLimit` "IT_AmmoR" 90))
    (:`then_4`
      (`self.ItemMapAddLimit` "IT_AmmoL" 20))
    (:`then_5`
      (`self.ItemMapAddLimit` "IT_GunR" 30))
    (:`then_6`
      (`self.ItemMapAddLimit` "IT_GunL" 10))))

(fn `UserConstructionScript`
  (`self.SetupMapAll`)
  (`self.CheckItem`))
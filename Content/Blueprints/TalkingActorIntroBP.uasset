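; Intro talking actor: a drone with a floating dialogue panel that opens and advances through talk entries for the player.
; Sphere overlaps report to DetectPlayer, while Interact calls NextTalkInput when text is visible and inventory and pickup checks pass.
; ShowTalkBP plays a timeline sizing the panel to runtime-built text components, which ChangeTalkBP rebuilds.
; Each tick, the panel faces the camera and the drone faces the player.
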(event `UpdateTextComponents`
  (bind _textcomponents (`self.TextComponents`))
  (bind _dialogueroot (`self.DialogueRoot`))
  (bind (_nextindex _lines) (break `TalkText` (`|GetArrayItem` (`self.Dialogue`) (`self.CurrentTalkIndex`))))
  (bind (_returnvalue_x _returnvalue_y) (`KismetMathLibrary.BreakVector` (`KismetMathLibrary.LessLess_VectorRotator` (- (`SceneComponent.RelativeLocation` (`self.BackgroundMesh`)) (`SceneComponent.RelativeLocation` _dialogueroot)) (`SceneComponent.K2_GetComponentRotation` _dialogueroot))))
  (if (> (`KismetArrayLibrary.Array_Length` _textcomponents) 0)
    (`|ExecutionSequence`
      (:`then_0`
        (for _array_element _textcomponents
          (`ActorComponent.K2_DestroyComponent` _array_element))
        (`KismetArrayLibrary.Array_Clear` _textcomponents))
      (:`then_1`
        (set `self.LongestLineLength` 0 :!label _label)
        (for (_array_element_2 _array_index) _lines
          (bind _returnvalue (`KismetStringLibrary.Len` _array_element_2))
          (if (> _returnvalue 0)
            (set `self.LongestLineLength` (`KismetMathLibrary.Max` _returnvalue (`self.LongestLineLength`)))
            (bind _returnvalue_2 (`AddComponent|NODE_AddTextRenderComponent-0` :`RelativeTransform` (`KismetMathLibrary.MakeTransform` (`KismetMathLibrary.MakeVector` 2.0 _returnvalue_y (+ (+ (* _array_index -20.0) (* (`KismetArrayLibrary.Array_Length` _lines) 10.0)) 10.0)))))
            (`/Engine/EditorBlueprintResources/StandardMacros.IsValid` _returnvalue_2
              (:`Is Valid`
                (`TextRenderComponent.K2_SetText` _returnvalue_2 (`KismetTextLibrary.Conv_StringToText` _array_element_2))
                (`SceneComponent.K2_AttachToComponent` _returnvalue_2 (`self.DialogueRoot`) "None" "KeepRelative" "KeepRelative" "KeepRelative" false)
                (`KismetArrayLibrary.Array_Add` (`self.TextComponents`) _returnvalue_2)))))))
    (else
      (goto _label))))

(event `self.ReceiveBeginPlay`
  (`self.EnableInput` (`GameplayStatics.GetPlayerController` 0))
  (`self.UpdateTextComponents`)
  (`self.ShowTextComponents` false)
  (`SceneComponent.SetAbsolute` (`self.TopBorder`) false false true)
  (`SceneComponent.SetAbsolute` (`self.BottomBorder`) false false true)
  (`SceneComponent.SetAbsolute` (`self.BottomRightCorner`) false false true)
  (`SceneComponent.SetAbsolute` (`self.BottomLeftCorner`) false false true)
  (`SceneComponent.SetAbsolute` (`self.TopRightCorner`) false false true)
  (`SceneComponent.SetAbsolute` (`self.TopLeftCorner`) false false true)
  (`SceneComponent.SetAbsolute` (`self.LeftBorder`) false false true)
  (`SceneComponent.SetAbsolute` (`self.RightBorder`) false false true)
  (`SceneComponent.SetAbsolute` (`self.InfoIcon`) false false true)
  (`SceneComponent.SetAbsolute` (`self.DroneBase`) false true true)
  (`SceneComponent.SetAbsolute` (`self.DialogueRoot`) false true true))

(event `self.ReceiveTick`
  (params (DeltaSeconds :type "Float (single-precision)"))
  (`self.TextLook`)
  (`self.DroneLook`))

(event `self.TalkSphereRange.OnComponentBeginOverlap`
  (params (OverlappedComponent :type "PrimitiveComponent Object Reference") (OtherActor :type "Actor Object Reference") (OtherComp :type "PrimitiveComponent Object Reference") (OtherBodyIndex :type Integer) (bFromSweep :type Boolean) (SweepResult :type "HitResult Structure (by ref)"))
  (cast `SurvivalWaveCharacter` OtherActor)
  (`self.DetectPlayer` true))

(event `self.ShowTalkBP`
  (params (bShowDialogue :type Boolean))
  (bind _infoicon (`self.InfoIcon`))
  (bind (_output_nextindex _output_lines) (break `TalkText` (`|GetArrayItem` (`self.Dialogue`) (`self.CurrentTalkIndex`))))
  (bind _returnvalue (* (`KismetMathLibrary.Conv_IntToDouble` (`self.LongestLineLength`)) 1.6))
  (bind _returnvalue_2 (* (`KismetArrayLibrary.Array_Length` _output_lines) 5.0))
  (bind _returnvalue_3 (+ _returnvalue (* _returnvalue (`self.BorderWidthPadding`))))
  (if bShowDialogue
    (bind (_direction _0to1) (`Timeline|ShowText` :!label _label_2)
      (:`Update`
        (`SceneComponent.K2_SetRelativeLocation` (`self.DialogueRoot`) (`KismetMathLibrary.VLerp` (`SceneComponent.RelativeLocation` (`self.NonTalkingArrow`)) (`SceneComponent.RelativeLocation` (`self.TalkingArrow`)) _0to1) false false)
        (`SceneComponent.SetRelativeScale3D` (`self.BackgroundMesh`) (`KismetMathLibrary.VLerp` (1.0 1.0 1.0) (`KismetMathLibrary.MakeVector` 1.0 _returnvalue_3 _returnvalue_2) _0to1))
        (`SceneComponent.SetRelativeScale3D` (`self.TopBorder`) (`KismetMathLibrary.VLerp` (1.0 1.0 1.0) (`KismetMathLibrary.MakeVector` 1.0 _returnvalue_3 1.0) _0to1))
        (`SceneComponent.SetRelativeScale3D` (`self.BottomBorder`) (`KismetMathLibrary.VLerp` (1.0 1.0 1.0) (`KismetMathLibrary.MakeVector` 1.0 _returnvalue_3 1.0) _0to1))
        (`SceneComponent.SetRelativeScale3D` (`self.LeftBorder`) (`KismetMathLibrary.VLerp` (1.0 1.0 1.0) (`KismetMathLibrary.MakeVector` 1.0 _returnvalue_2 1.0) _0to1))
        (`SceneComponent.SetRelativeScale3D` (`self.RightBorder`) (`KismetMathLibrary.VLerp` (1.0 1.0 1.0) (`KismetMathLibrary.MakeVector` 1.0 _returnvalue_2 1.0) _0to1))
        (`SceneComponent.K2_SetRelativeLocation` _infoicon (`KismetMathLibrary.MakeVector` 1.0 0.0 (`KismetMathLibrary.Lerp` -10.0 10.0 _0to1)) false false)
        (`SceneComponent.K2_SetRelativeRotation` _infoicon (`KismetMathLibrary.MakeRotator` (`KismetMathLibrary.Lerp` 0.0 180.0 _0to1)) false false))
      (:`Finished`
        (if (`|EnumEquality` _direction "Forward")
          (`self.ShowTextComponents` true)
          (set `self.bTextVisible` true))))
    (else
      (set `self.bTextVisible` false)
      (`self.ShowTextComponents` false)
      (goto _label_2 :!via `Reverse`))))

(event `InputAction|Interact` :consume false
  (params (Key :type "Key Structure"))
  (:`Pressed`
    (if (`self.bTextVisible`)
      (bind _assurvival_wave_character (cast `SurvivalWaveCharacter` (`GameplayStatics.GetPlayerCharacter` 0)))
      (bind _returnvalue (`SurvivalWaveCharacter.GetInventory` _assurvival_wave_character))
      (bind _returnvalue_2 (`SurvivalWaveCharacter.GetPickup` _assurvival_wave_character))
      (if (and (not _returnvalue) (<= (`.quantity` (break `Item` _returnvalue_2)) -1))
        (`self.NextTalkInput`)))))

(event `self.TalkSphereRange.OnComponentEndOverlap`
  (params (OverlappedComponent :type "PrimitiveComponent Object Reference") (OtherActor :type "Actor Object Reference") (OtherComp :type "PrimitiveComponent Object Reference") (OtherBodyIndex :type Integer))
  (cast `SurvivalWaveCharacter` OtherActor)
  (`self.DetectPlayer` false))

(event `ShowTextComponents`
  (params (Show :type Boolean))
  (for _array_element (`self.TextComponents`)
    (`SceneComponent.SetHiddenInGame` _array_element (not Show) false)))

(event `TextLook`
  (bind _assurvival_wave_character (cast `SurvivalWaveCharacter` (`GameplayStatics.GetPlayerCharacter` 0)))
  (`/Engine/EditorBlueprintResources/StandardMacros.IsValid` _assurvival_wave_character
    (:`Is Valid`
      (`SceneComponent.K2_SetRelativeRotation` (`self.DialogueRoot`) (`KismetMathLibrary.FindLookAtRotation` (`SceneComponent.K2_GetComponentLocation` (`self.DialogueRoot`)) (`SceneComponent.K2_GetComponentLocation` (`SurvivalWaveCharacter.FollowCamera` _assurvival_wave_character))) false false))))

(event `self.ChangeTalkBP`
  (bind _btextvisible (`self.bTextVisible`))
  (`KismetSystemLibrary.PrintString` "Hello")
  (`self.UpdateTextComponents`)
  (`self.ShowTextComponents` _btextvisible)
  (`self.ShowTalkBP` _btextvisible))

(event `DroneLook`
  (bind _assurvival_wave_character (cast `SurvivalWaveCharacter` (`GameplayStatics.GetPlayerCharacter` 0)))
  (`/Engine/EditorBlueprintResources/StandardMacros.IsValid` _assurvival_wave_character
    (:`Is Valid`
      (`SceneComponent.K2_SetRelativeRotation` (`self.DroneBase`) (`KismetMathLibrary.FindLookAtRotation` (`SceneComponent.K2_GetComponentLocation` (`self.DroneBase`)) (+ (`self.K2_GetActorLocation` _assurvival_wave_character) (0.0 0.0 50.0))) false false))))

(fn `UserConstructionScript`)
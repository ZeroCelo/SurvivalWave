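; DemoWaveMode is the game mode Blueprint for the survival wave demo, handling room streaming, game end and the death camera.
; BeginPlay sets game-only input and flags the game instance as in-game, while LoadLevel and UnLoadLevel stream levels by name.
; GameEnd prints a state-based debug message and returns to MainMenuPersist.
; DeathAnim uses a timeline to lift the player's camera boom and turn the camera toward the character mesh.
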(event `self.ReceiveBeginPlay`
  (`WidgetBlueprintLibrary.SetInputMode_GameOnly` (`GameplayStatics.GetPlayerController` 0))
  (bind _aswave_game_instance (cast `/Game/Blueprints/GameInstance/WaveGameInstance` (`GameplayStatics.GetGameInstance`)))
  (set `/Game/Blueprints/GameInstance/WaveGameInstance.InGame` true _aswave_game_instance))

(event `self.UnLoadLevel`
  (params (CurrentRoom :type Integer) (level :type String))
  (`GameplayStatics.UnloadStreamLevel` (`KismetStringLibrary.Conv_StringToName` level)))

(event `self.LoadLevel`
  (params (CurrentRoom :type Integer) (level :type String))
  (`|ExecutionSequence`
    (:`then_0`
      (`GameplayStatics.LoadStreamLevel` (`KismetStringLibrary.Conv_StringToName` level) true)
      (set `self.bLastRoomLoad` true))))

(event `self.GameEnd`
  (if (`|EnumEquality` (`self.GetCurrentState`) "EGameOver")
    (`KismetSystemLibrary.PrintString` "Deu Ruim pro player")
    (else
      (`KismetSystemLibrary.PrintString` "Player ta de boas")))
  (`GameplayStatics.OpenLevel` "MainMenuPersist"))

(event `self.DeathAnim`
  (bind (_direction _position _rotate) (`Timeline|Death`)
    (:`Update`
      (bind _assurvival_wave_character (cast `SurvivalWaveCharacter` (`GameplayStatics.GetPlayerCharacter` 0)))
      (bind _cameraboom (`SurvivalWaveCharacter.CameraBoom` _assurvival_wave_character))
      (`SceneComponent.K2_SetRelativeLocation` _cameraboom (`KismetMathLibrary.VLerp` (`SceneComponent.RelativeLocation` _cameraboom) (0.0 0.0 400.0) _position) false false)
      (bind _followcamera (`SurvivalWaveCharacter.FollowCamera` _assurvival_wave_character))
      (`SceneComponent.K2_SetWorldRotation` _followcamera (`KismetMathLibrary.RLerp` (`SceneComponent.K2_GetComponentRotation` _followcamera) (`KismetMathLibrary.FindLookAtRotation` (`SceneComponent.K2_GetComponentLocation` _followcamera) (`SceneComponent.K2_GetComponentLocation` (`Character.Mesh` _assurvival_wave_character))) _rotate) false false))))

(fn `UserConstructionScript`)
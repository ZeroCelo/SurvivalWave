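; Main menu player display actor that shows a mannequin holding a weapon, tinted with the player color stored in WaveGameInstance.
; The construction script creates a dynamic dissolve material on the skeletal mesh, sets its dissolve amount and body color, and attaches the weapon mesh to the right-hand socket.
; Tick re-reads the game instance color every frame and pushes it to the material, keeping the preview in sync with color changes.
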(event `self.ReceiveTick`
  (params (DeltaSeconds :type "Float (single-precision)"))
  (bind _aswave_game_instance (cast `/Game/Blueprints/GameInstance/WaveGameInstance` (`GameplayStatics.GetGameInstance`)))
  (`MaterialInstanceDynamic.SetVectorParameterValue` (`self.MatRef`) "BodyColor" (`/Game/Blueprints/GameInstance/WaveGameInstance.PlayerColor` _aswave_game_instance)))

(fn `UserConstructionScript`
  (`|ExecutionSequence`
    (:`then_0`
      (bind _returnvalue (`PrimitiveComponent.CreateDynamicMaterialInstance` (`self.SkeletalMesh`) 0 "/Game/Materials/DissolveMannequin.DissolveMannequin"))
      (set `self.MatRef` _returnvalue)
      (`MaterialInstanceDynamic.SetScalarParameterValue` (`self.MatRef`) "Dissolve" -0.2)
      (bind _aswave_game_instance (cast `/Game/Blueprints/GameInstance/WaveGameInstance` (`GameplayStatics.GetGameInstance`)))
      (`MaterialInstanceDynamic.SetVectorParameterValue` (`self.MatRef`) "BodyColor" (`/Game/Blueprints/GameInstance/WaveGameInstance.PlayerColor` _aswave_game_instance)))
    (:`then_1`
      (`SceneComponent.K2_AttachToComponent` (`self.WeaponMesh`) (`self.SkeletalMesh`) "SockHandRight" "KeepRelative" "KeepRelative" "KeepRelative" true))))
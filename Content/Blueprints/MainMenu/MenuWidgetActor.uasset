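; Main menu actor that hides and shows the menu by rotating its MainMenuArrow component.
; On BeginPlay it caches the arrow's roll and yaw.
; HideMainMenu plays the HideMain timeline, driving the arrow's pitch up to 180 degrees times the Rotate track while keeping the cached roll and yaw.
; ShowMainMenu reverses that timeline from the end to swing it back.
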(event `self.ReceiveBeginPlay`
  (bind (_relativerotation_roll _relativerotation_pitch _relativerotation_yaw) (`KismetMathLibrary.BreakRotator` (`SceneComponent.RelativeRotation` (`self.MainMenuArrow`))))
  (set `self.MainMenuRotX` _relativerotation_roll)
  (set `self.MainMenuRotZ` _relativerotation_yaw))

(event `HideMainMenu`
  (bind (_direction _rotate) (`Timeline|HideMain` :!via `PlayFromStart` :!label _label)
    (:`Update`
      (`SceneComponent.K2_SetRelativeRotation` (`self.MainMenuArrow`) (`KismetMathLibrary.MakeRotator` (`self.MainMenuRotX`) (* _rotate 180.0) (`self.MainMenuRotZ`)) false false))))

(event `ShowMainMenu`
  (goto _label :!via `ReverseFromEnd`))

(fn `UserConstructionScript`)
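; DroneMenu is a main menu drone actor that plays a continuous procedural hover animation on its Sphere component.
; Three self-restarting timelines start on BeginPlay, driving vertical bob, sideways strafe and roll, each scaled by its own amplitude variable.
; They write into shared relative position and rotation variables, which Tick applies to the Sphere, so the motions combine independently.
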(event `self.ReceiveBeginPlay`
  (`self.AnimateFly`)
  (`self.AnimateStrafe`)
  (`self.AnimateRotate`))

(event `self.ReceiveTick`
  (params (DeltaSeconds :type "Float (single-precision)"))
  (`SceneComponent.K2_SetRelativeLocation` (`self.Sphere`) (`self.DroneRelativePos`) false false)
  (`SceneComponent.K2_SetRelativeRotation` (`self.Sphere`) (`self.DroneRelativeRot`) false false))

(event `AnimateFly`
  (bind (_dronerelativepos_x _dronerelativepos_y) (`KismetMathLibrary.BreakVector` (`self.DroneRelativePos`)))
  (bind (_direction _driver) (`Timeline|Fly` :!via `PlayFromStart`)
    (:`Update`
      (set `self.DroneRelativePos` (`KismetMathLibrary.MakeVector` _dronerelativepos_x _dronerelativepos_y (* _driver (`self.FlyHeight`)))))
    (:`Finished`
      (`self.AnimateFly`))))

(event `AnimateStrafe`
  (bind (_dronerelativepos_x _dronerelativepos_y _dronerelativepos_z) (`KismetMathLibrary.BreakVector` (`self.DroneRelativePos`)))
  (bind (_direction _translate) (`Timeline|Strafe` :!via `PlayFromStart`)
    (:`Update`
      (set `self.DroneRelativePos` (`KismetMathLibrary.MakeVector` _dronerelativepos_x (* _translate (`self.FlyStrafe`)) _dronerelativepos_z)))
    (:`Finished`
      (`self.AnimateStrafe`))))

(event `AnimateRotate`
  (bind (_dronerelativerot_roll _dronerelativerot_pitch _dronerelativerot_yaw) (`KismetMathLibrary.BreakRotator` (`self.DroneRelativeRot`)))
  (bind (_direction _rotate) (`Timeline|Rotate` :!via `PlayFromStart`)
    (:`Update`
      (set `self.DroneRelativeRot` (`KismetMathLibrary.MakeRotator` (* _rotate (`self.FlyRotate`)) _dronerelativerot_pitch _dronerelativerot_yaw)))
    (:`Finished`
      (`self.AnimateRotate`))))

(fn `UserConstructionScript`)
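; Main menu game mode that drives a 3D menu through camera transitions and a spawned MenuWidgetActor.
; On BeginPlay it finds level cameras by their first tag, cuts to the loading camera, blends to the main one, and enables cursor input.
; Events blend between options, graphics and help cameras, forward menu visibility to the widget actor or WaveGameInstance, and open the DemoPersist level from the loading view.
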(event `self.ReceiveBeginPlay`
  (bind _returnvalue (`GameplayStatics.GetPlayerController` 0))
  (`|SpawnActorFromClass` "/Game/Blueprints/MainMenu/MenuWidgetActor.MenuWidgetActor_C" (`KismetMathLibrary.MakeTransform` (0.0 0.0 0.0)) "Undefined" "OverrideRootScale" null null)
  (`self.FindCameras`)
  (`self.FindMenuActor`)
  (`self.SwitchLoadingCam`)
  (`KismetSystemLibrary.Delay` 0.3)
  (`self.SwitchMainCam`)
  (`WidgetBlueprintLibrary.SetInputMode_GameAndUIEx` _returnvalue null "DoNotLock" false)
  (set `PlayerController.bShowMouseCursor` true _returnvalue)
  (bind _aswave_game_instance (cast `/Game/Blueprints/GameInstance/WaveGameInstance` (`GameplayStatics.GetGameInstance`)))
  (set `/Game/Blueprints/GameInstance/WaveGameInstance.InGame` false _aswave_game_instance))

(event `FindMenuActor`
  (bind _outactors (`GameplayStatics.GetAllActorsOfClass` "/Game/Blueprints/MainMenu/MenuWidgetActor.MenuWidgetActor_C"))
  (for _array_element _outactors
    (set `self.WidgetActor` _array_element)))

(event `FindCameras`
  (bind _outactors (`GameplayStatics.GetAllActorsOfClass` "/Script/Engine.CameraActor"))
  (for _array_element _outactors
    (bind _tags (`Actor.Tags` _array_element))
    (if (> (`KismetArrayLibrary.Array_Length` _tags) 0)
      (switch `name` (`|GetArrayItem` _tags)
        (:`MainMenuCam`
          (set `self.MainMenuCam` _array_element))
        (:`OptionsCam`
          (set `self.OptionsMenuCam` _array_element))
        (:`LoadingCam`
          (set `self.LoadingCam` _array_element))
        (:`VisualCam`
          (set `self.GraphicsCam` _array_element))
        (:`HelpCam`
          (set `self.HelpCam` _array_element))))))

(event `SwitchMainCam`
  (if (`KismetSystemLibrary.IsValid` (`self.MainMenuCam`))
    (`PlayerController.SetViewTargetWithBlend` (`GameplayStatics.GetPlayerController` 0) (`self.MainMenuCam`) 1.0 "VTBlend_EaseIn" 1.0 true)))

(event `ShowMainMenu`
  (bind _widgetactor (`self.WidgetActor`))
  (if (`KismetSystemLibrary.IsValid` _widgetactor)
    (`/Game/Blueprints/MainMenu/MenuWidgetActor.ShowMainMenu` _widgetactor)))

(event `HideMainMenu`
  (bind _widgetactor (`self.WidgetActor`))
  (if (`KismetSystemLibrary.IsValid` _widgetactor)
    (`/Game/Blueprints/MainMenu/MenuWidgetActor.HideMainMenu` _widgetactor)))

(event `SwitchOptionsCam`
  (if (`KismetSystemLibrary.IsValid` (`self.OptionsMenuCam`))
    (`PlayerController.SetViewTargetWithBlend` (`GameplayStatics.GetPlayerController` 0) (`self.OptionsMenuCam`) 1.0 "VTBlend_EaseIn" 1.0 true)))

(event `StartDemo`
  (`self.SwitchLoadingCam`)
  (`KismetSystemLibrary.Delay` 0.2)
  (`GameplayStatics.OpenLevel` "DemoPersist"))

(event `ShowGraphics`
  (`self.SwitchGraphicsCam`)
  (bind _aswave_game_instance (cast `/Game/Blueprints/GameInstance/WaveGameInstance` (`GameplayStatics.GetGameInstance`)))
  (`/Game/Blueprints/GameInstance/WaveGameInstance.ShowVisualMenu` _aswave_game_instance))

(event `SwitchLoadingCam`
  (if (`KismetSystemLibrary.IsValid` (`self.LoadingCam`))
    (`PlayerController.SetViewTargetWithBlend` (`GameplayStatics.GetPlayerController` 0) (`self.LoadingCam`) 0.0 "VTBlend_EaseIn" 1.0 true)))

(event `HideGraphics`
  (`self.SwitchOptionsCam`))

(event `SwitchGraphicsCam`
  (if (`KismetSystemLibrary.IsValid` (`self.GraphicsCam`))
    (`PlayerController.SetViewTargetWithBlend` (`GameplayStatics.GetPlayerController` 0) (`self.GraphicsCam`) 1.0 "VTBlend_EaseIn" 1.0 true)))

(event `ShowHelp`
  (bind _aswave_game_instance (cast `/Game/Blueprints/GameInstance/WaveGameInstance` (`GameplayStatics.GetGameInstance`)))
  (`/Game/Blueprints/GameInstance/WaveGameInstance.ShowHelpMenu` _aswave_game_instance)
  (`self.SwitchHelpCam`))

(event `SwitchHelpCam`
  (if (`KismetSystemLibrary.IsValid` (`self.HelpCam`))
    (`PlayerController.SetViewTargetWithBlend` (`GameplayStatics.GetPlayerController` 0) (`self.HelpCam`) 1.0 "VTBlend_EaseIn" 1.0 true)))

(fn `UserConstructionScript`)
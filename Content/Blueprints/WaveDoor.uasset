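; WaveDoor is a two-panel sliding door with a lock emblem that shows whether it is locked, waiting or open to use.
; OpenDoor only works while the door is active, playing the Opening timeline to slide the panels apart and roll the lock.
; CloseDoor reverses that timeline, which marks the door closed and calls SetupActive when finished.
; SetupActive picks the lock material from IsDoorActive and IsDoorWaiting.
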(event `self.OpenDoor`
  (bind _returnvalue (`self.IsDoorActive`))
  (if _returnvalue
    (`PrimitiveComponent.SetMaterial` (`self.Lock`) 0 "/Game/DemoRoom/Materials/M_UE4_Logo_Doors.M_UE4_Logo_Doors")
    (set `self.bDoorClosed` false)
    (bind (_direction _move _rotate) (`Timeline|Opening` :!label _label)
      (:`Update`
        (`|ExecutionSequence`
          (:`then_0`
            (bind _returnvalue_2 (* _move 200.0))
            (`SceneComponent.K2_SetRelativeLocation` (`self.LeftDoor`) (`KismetMathLibrary.MakeVector` 0.0 _returnvalue_2) false false)
            (`SceneComponent.K2_SetRelativeLocation` (`self.RightDoor`) (`KismetMathLibrary.MakeVector` 0.0 (* _returnvalue_2 -1.0)) false false))
          (:`then_1`
            (`SceneComponent.K2_SetRelativeRotation` (`self.Lock`) (`KismetMathLibrary.MakeRotator` (* _rotate 90.0)) false false))))
      (:`Finished`
        (if (`|EnumEquality` _direction "Backward")
          (`self.SetupActive`)
          (set `self.bDoorClosed` true))))))

(event `self.CloseDoor`
  (goto _label :!via `Reverse`))

(event `self.SetupActive`
  (bind _lock (`self.Lock`))
  (bind _returnvalue (`self.IsDoorActive`))
  (if _returnvalue
    (bind _returnvalue_2 (`self.IsDoorWaiting`))
    (if (not _returnvalue_2)
      (`PrimitiveComponent.SetMaterial` _lock 0 "/Game/DemoRoom/Materials/M_UE4_Logo_Door_Open.M_UE4_Logo_Door_Open")
      (else
        (`PrimitiveComponent.SetMaterial` _lock 0 "/Game/DemoRoom/Materials/M_UE4_Logo_DoorsWaiting.M_UE4_Logo_DoorsWaiting")))
    (else
      (`PrimitiveComponent.SetMaterial` _lock 0 "/Game/DemoRoom/Materials/M_UE4_Logo_Door_Lock.M_UE4_Logo_Door_Lock"))))

(fn `UserConstructionScript`)
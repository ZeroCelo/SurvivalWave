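; RoomBP is a modular room actor whose four side walls (X+, X-, Y+, Y-) are configured individually through boolean flags.
; The Construction Script calls one switch event per side, which either hides the wall and disables its collision or picks a room wall or demo divider mesh.
; The Y+ side also sets a different relative transform for each mesh.
; BeginPlay, Tick and overlap events are unused.
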(event `SwitchWallXPos`
  (bind _wall_xpos (`self.Wall_XPos`))
  (if (`self.WallXPosNull`)
    (`SceneComponent.SetVisibility` _wall_xpos false false)
    (`PrimitiveComponent.SetCollisionEnabled` _wall_xpos "NoCollision")
    (elif (`self.WallXPos`)
      (`StaticMeshComponent.SetStaticMesh` _wall_xpos "/Game/DemoRoom/Meshes/SM_URoom_Wall.SM_URoom_Wall")
      (else
        (`StaticMeshComponent.SetStaticMesh` _wall_xpos "/Game/DemoRoom/Meshes/SM_DemoDivider_1.SM_DemoDivider_1")))))

(event `SwitchWallXNeg`
  (bind _wall_xneg (`self.Wall_XNeg`))
  (if (`self.WallXNegNull`)
    (`SceneComponent.SetVisibility` _wall_xneg false false)
    (`PrimitiveComponent.SetCollisionEnabled` _wall_xneg "NoCollision")
    (elif (`self.WallXNeg`)
      (`StaticMeshComponent.SetStaticMesh` _wall_xneg "/Game/DemoRoom/Meshes/SM_URoom_Wall.SM_URoom_Wall")
      (else
        (`StaticMeshComponent.SetStaticMesh` _wall_xneg "/Game/DemoRoom/Meshes/SM_DemoDivider_1.SM_DemoDivider_1")))))

(event `SwitchWallYPos`
  (bind _wall_ypos (`self.Wall_YPos`))
  (bind _wall_ypos_2 (`self.Wall_YPos`))
  (if (`self.WallYPosNull`)
    (`SceneComponent.SetVisibility` _wall_ypos false false)
    (`PrimitiveComponent.SetCollisionEnabled` _wall_ypos "NoCollision")
    (elif (`self.WallYPos`)
      (`StaticMeshComponent.SetStaticMesh` _wall_ypos "/Game/DemoRoom/Meshes/SM_URoom_Wall.SM_URoom_Wall")
      (`SceneComponent.K2_SetRelativeTransform` _wall_ypos_2 (`KismetMathLibrary.MakeTransform` (0.0 -850.0 0.0) (struct :`Yaw` 180.0)) false false)
      (else
        (`StaticMeshComponent.SetStaticMesh` _wall_ypos "/Game/DemoRoom/Meshes/SM_DemoDivider_1.SM_DemoDivider_1")
        (`SceneComponent.K2_SetRelativeTransform` _wall_ypos_2 (`KismetMathLibrary.MakeTransform` (0.0 1050.0 0.0)) false false)))))

(event `SwitchWallYNeg`
  (bind _wall_yneg (`self.Wall_YNeg`))
  (if (`self.WallYNegNull`)
    (`SceneComponent.SetVisibility` _wall_yneg false false)
    (`PrimitiveComponent.SetCollisionEnabled` _wall_yneg "NoCollision")
    (elif (`self.WallYNeg`)
      (`StaticMeshComponent.SetStaticMesh` _wall_yneg "/Game/DemoRoom/Meshes/SM_URoom_Wall.SM_URoom_Wall")
      (else
        (`StaticMeshComponent.SetStaticMesh` _wall_yneg "/Game/DemoRoom/Meshes/SM_DemoDivider_1.SM_DemoDivider_1")))))

(fn `UserConstructionScript`
  (`self.SwitchWallXPos`)
  (`self.SwitchWallXNeg`)
  (`self.SwitchWallYPos`)
  (`self.SwitchWallYNeg`))
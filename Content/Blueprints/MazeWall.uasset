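; MazeWall is a maze wall that stays hidden in game until something overlaps its surrounding trigger box, feeding a player-centred sphere mask to its material.
; The construction script creates the tiled dynamic material, pads the box horizontally by the sphere radius and centres the sphere on the wall outside play.
; While overlapped, a looping timer writes the player's location into the material; end overlap clears it and hides the wall.
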(event `self.ReceiveBeginPlay`
  (set `self.Playing` true)
  (`MaterialInstanceDynamic.SetScalarParameterValue` (`self.WallMat`) "SphereRadius" (`self.SphereRadius`))
  (`self.UpdateSphere`)
  (`SceneComponent.SetHiddenInGame` (`self.Wall`) true false))

(event `UpdateSphere`
  (`MaterialInstanceDynamic.SetVectorParameterValue` (`self.WallMat`) "SphereCenter" (`KismetMathLibrary.Conv_VectorToLinearColor` (`self.K2_GetActorLocation` (`GameplayStatics.GetPlayerCharacter` 0)))))

(event `self.Box.OnComponentBeginOverlap`
  (params (OverlappedComponent :type "PrimitiveComponent Object Reference") (OtherActor :type "Actor Object Reference") (OtherComp :type "PrimitiveComponent Object Reference") (OtherBodyIndex :type Integer) (bFromSweep :type Boolean) (SweepResult :type "HitResult Structure (by ref)"))
  (`KismetSystemLibrary.K2_SetTimerDelegate` (delegate `UpdateSphere`) 0.05 true)
  (`SceneComponent.SetHiddenInGame` (`self.Wall`) false false))

(event `self.Box.OnComponentEndOverlap`
  (params (OverlappedComponent :type "PrimitiveComponent Object Reference") (OtherActor :type "Actor Object Reference") (OtherComp :type "PrimitiveComponent Object Reference") (OtherBodyIndex :type Integer))
  (`KismetSystemLibrary.K2_SetTimerDelegate` (delegate `UpdateSphere`))
  (`SceneComponent.SetHiddenInGame` (`self.Wall`) true false))

(fn `UserConstructionScript`
  (bind _wallmat (`self.WallMat`))
  (bind _box (`self.Box`))
  (bind _sphereradius (`self.SphereRadius`))
  (bind (_origin _boxextent) (`KismetSystemLibrary.GetComponentBounds` (`self.Wall`)))
  (bind (_returnvalue_x _returnvalue_y _returnvalue_z) (`KismetMathLibrary.BreakVector` (`KismetMathLibrary.GreaterGreater_VectorRotator` _boxextent (`self.K2_GetActorRotation`))))
  (bind _returnvalue (`PrimitiveComponent.CreateDynamicMaterialInstance` (`self.Wall`) 0 null))
  (set `self.WallMat` _returnvalue)
  (`MaterialInstanceDynamic.SetScalarParameterValue` _wallmat "TileX" (`self.TileX`))
  (`MaterialInstanceDynamic.SetScalarParameterValue` _wallmat "TileY" (`self.TileY`))
  (`SceneComponent.SetAbsolute` _box false false true)
  (`BoxComponent.SetBoxExtent` _box (`KismetMathLibrary.MakeVector` (+ _sphereradius _returnvalue_x) (+ _sphereradius _returnvalue_y) _returnvalue_z) false)
  (if (not (`self.Playing`))
    (`MaterialInstanceDynamic.SetVectorParameterValue` (`self.WallMat`) "SphereCenter" (`KismetMathLibrary.Conv_VectorToLinearColor` _origin))))
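; Survival character Blueprint that carries two test weapons and forwards character state to its animation Blueprint.
; BeginPlay spawns both weapons on hand and holster sockets, stores them in the Weapon array, then calls AnimNotifyEquipEnd on SurvivalAnim_BP.
; SwitchGunBP re-attaches the weapons between sockets according to WeaponSelect.
; Separate update events copy the running, aiming, firing and switching flags into SurvivalAnim_BP, with no Tick polling.
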(event `self.ReceiveBeginPlay`
  (bind _mesh (`self.Mesh`))
  (bind _returnvalue (`|SpawnActorFromClass` "/Game/Blueprints/WeaponTest_BP.WeaponTest_BP_C" (`SceneComponent.GetSocketTransform` _mesh "HandRightSock1" "RTS_World") "Undefined" "OverrideRootScale"))
  (`self.K2_AttachToComponent` _returnvalue (`self.Mesh`) "HandRightSock1" "KeepWorld" "KeepWorld" "KeepRelative" true)
  (`KismetArrayLibrary.Array_Set` (`self.Weapon`) 1 _returnvalue)
  (bind _returnvalue_2 (`|SpawnActorFromClass` "/Game/Blueprints/WeaponTest2_BP.WeaponTest2_BP_C" (`SceneComponent.GetSocketTransform` _mesh "Weapon2" "RTS_World") "Undefined" "OverrideRootScale"))
  (`self.K2_AttachToComponent` _returnvalue_2 (`self.Mesh`) "Weapon2" "KeepWorld" "KeepWorld" "KeepRelative" true)
  (`KismetArrayLibrary.Array_Set` (`self.Weapon`) 2 _returnvalue_2)
  (bind _assurvival_anim_bp (cast `/Game/Animations/SurvivalAnim_BP` (`SkeletalMeshComponent.GetAnimInstance` (`self.Mesh`))))
  (`/Game/Animations/SurvivalAnim_BP.AnimNotify_EquipEnd` _assurvival_anim_bp))

(event `self.UpdateAnimRun`
  (bind _assurvival_anim_bp (cast `/Game/Animations/SurvivalAnim_BP` (`SkeletalMeshComponent.GetAnimInstance` (`self.Mesh`))))
  (set `/Game/Animations/SurvivalAnim_BP.Running` (`self.running`) _assurvival_anim_bp))

(event `self.SwitchGunBP`
  (bind _mesh (`self.Mesh`))
  (bind _mesh_2 (`self.Mesh`))
  (bind _weapon (`self.Weapon`))
  (if (== (`self.weapon_select`) 1)
    (`self.K2_AttachToComponent` (`KismetArrayLibrary.Array_Get` _weapon 2) _mesh "Weapon2" "KeepRelative" "KeepRelative" "KeepRelative" true)
    (`self.K2_AttachToComponent` (`KismetArrayLibrary.Array_Get` _weapon 1) _mesh_2 "HandRightSock1" "KeepRelative" "KeepRelative" "KeepRelative" true)
    (else
      (`self.K2_AttachToComponent` (`KismetArrayLibrary.Array_Get` _weapon 1) _mesh "Weapon1" "KeepRelative" "KeepRelative" "KeepRelative" true)
      (`self.K2_AttachToComponent` (`KismetArrayLibrary.Array_Get` _weapon 2) _mesh_2 "HandRightSock1" "KeepRelative" "KeepRelative" "KeepRelative" true))))

(event `self.UpdateAnimAim`
  (bind _assurvival_anim_bp (cast `/Game/Animations/SurvivalAnim_BP` (`SkeletalMeshComponent.GetAnimInstance` (`self.Mesh`))))
  (set `/Game/Animations/SurvivalAnim_BP.Aiming` (`self.aiming`) _assurvival_anim_bp))

(event `self.ReceiveTick`
  (params (DeltaSeconds :type "Float (single-precision)")))

(event `self.UpdateAnimFire`
  (bind _assurvival_anim_bp (cast `/Game/Animations/SurvivalAnim_BP` (`SkeletalMeshComponent.GetAnimInstance` (`self.Mesh`))))
  (set `/Game/Animations/SurvivalAnim_BP.Firing` (`self.firing`) _assurvival_anim_bp))

(event `self.UpdateAnimSwitch`
  (bind _assurvival_anim_bp (cast `/Game/Animations/SurvivalAnim_BP` (`SkeletalMeshComponent.GetAnimInstance` (`self.Mesh`))))
  (set `/Game/Animations/SurvivalAnim_BP.Switchin` (`self.switching`) _assurvival_anim_bp))

(fn `UserConstructionScript`)
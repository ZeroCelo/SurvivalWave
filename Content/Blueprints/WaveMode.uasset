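; WaveMode is a Blueprint for a room-based wave mode that currently handles level streaming and a stubbed game end.
; LoadLevel streams a named level in without blocking and shows it once loaded, while UnLoadLevel streams one out.
; GameEnd only prints a Portuguese placeholder noting that the stage should exit there.
; The WaveRooms index check and the FindDoors and FindSpawners calls are disconnected and never run.
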(event `self.UnLoadLevel`
  (params (CurrentRoom :type Integer) (level :type String))
  (`GameplayStatics.UnloadStreamLevel` (`KismetStringLibrary.Conv_StringToName` level)))

(event `self.LoadLevel`
  (params (CurrentRoom :type Integer) (level :type String))
  (`|ExecutionSequence`
    (:`then_0`
      (`GameplayStatics.LoadStreamLevel` (`KismetStringLibrary.Conv_StringToName` level) true))))

(event `self.GameEnd`
  (`KismetSystemLibrary.PrintString` "Aqui deveria sair da fase"))

(fn `UserConstructionScript`)